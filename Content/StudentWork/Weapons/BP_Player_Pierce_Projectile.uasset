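; Player piercing projectile that damages each actor its mesh overlaps and can pass through several before being destroyed.
; Each overlap applies fixed damage and increments a hit counter; reaching MaxCount spawns a Niagara impact effect and destroys the projectile.
; Earlier hits set a short life timer that destroys it without the effect, so this graph only starts that timeout after a first overlap.
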(event OnComponentBeginOverlap(ProjectileMesh)
  (params (OverlappedComponent :type Primitive%20Component%20Object%20Reference) (OtherActor :type Actor%20Object%20Reference) (OtherComp :type Primitive%20Component%20Object%20Reference) (OtherBodyIndex :type Integer) (bFromSweep :type Boolean) (SweepResult :type Hit%20Result%20Structure%20%28by%20ref%29))
  (bind _returnvalue (Transformation|GetActorTransform))
  (Variables|Default|SetCounter (+ 1.0 (Variables|Default|GetCounter)))
  (Game|Damage|ApplyDamage OtherActor 2e+01 0 0)
  (if (== (Variables|Default|GetCounter) (Variables|Default|GetMaxCount))
    (Niagara|SpawnSystematLocation "/Game/StudentWork/Effects/NS_Player_ProjectileImpact.NS_Player_ProjectileImpact" (.location _returnvalue) (.rotation _returnvalue))
    (Actor|DestroyActor)
    (else
      (Utilities|Time|SetTimerbyEvent (delegate Custom|Life%20Timer) 2.0))))

(event Custom|Life%20Timer
  (Actor|DestroyActor))

(fn ConstructionScript)