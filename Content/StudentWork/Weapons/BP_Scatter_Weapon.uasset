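; BP_Scatter_Weapon is a tank weapon that fires a scatter shot of three player projectiles.
; When triggered off cooldown, it plays a firing sound and spawns a BP_Player_Scatter_Projectile at each of the owning tank's three direction arrows, using their location and rotation.
; It then sets a cooldown flag that a short timer clears, limiting the fire rate.
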(event Custom|End%20Cool%20Down
  (Variables|Default|SetCool%20Down false))

(event EventTriggered
  (bind _mytank (Variables|Default|GetMyTank))
  (bind _directionarrow1 (Variables|/Game/Blueprints/BP_PlayerCharacter.BP_PlayerCharacter_C|GetDirectionArrow1 _mytank))
  (bind _directionarrow (Variables|/Game/Blueprints/BP_PlayerCharacter.BP_PlayerCharacter_C|GetDirectionArrow _mytank))
  (bind _directionarrow2 (Variables|/Game/Blueprints/BP_PlayerCharacter.BP_PlayerCharacter_C|GetDirectionArrow2 _mytank))
  (bind _returnvalue (Transformation|GetWorldLocation _directionarrow))
  (if (not (Variables|Default|GetCool%20Down))
    (Audio|PlaySoundatLocation "/Game/StudentWork/Effects/SFX/mixkit-falling-on-foil-748.mixkit-falling-on-foil-748" _returnvalue "0, 0, 0" 1.0 1.0 0.0 0 0 0 0)
    (Game|SpawnActorfromClass "/Game/StudentWork/Weapons/BP_Player_Scatter_Projectile.BP_Player_Scatter_Projectile_C" (Math|Transform|MakeTransform _returnvalue (Transformation|GetWorldRotation _directionarrow) "1.000000,1.000000,1.000000") "Undefined" "MultiplyWithRoot" 0 0)
    (Game|SpawnActorfromClass "/Game/StudentWork/Weapons/BP_Player_Scatter_Projectile.BP_Player_Scatter_Projectile_C" (Math|Transform|MakeTransform (Transformation|GetWorldLocation _directionarrow1) (Transformation|GetWorldRotation _directionarrow1) "1.000000,1.000000,1.000000") "Undefined" "MultiplyWithRoot" 0 0)
    (Game|SpawnActorfromClass "/Game/StudentWork/Weapons/BP_Player_Scatter_Projectile.BP_Player_Scatter_Projectile_C" (Math|Transform|MakeTransform (Transformation|GetWorldLocation _directionarrow2) (Transformation|GetWorldRotation _directionarrow2) "1.000000,1.000000,1.000000") "Undefined" "MultiplyWithRoot" 0 0)
    (Variables|Default|SetCool%20Down true)
    (Utilities|Time|SetTimerbyEvent (delegate Custom|End%20Cool%20Down) 1.4)))

(fn ConstructionScript
  (|CallParentFunction))