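; Bubble weapon Blueprint that fires player bubble projectiles from the owning tank.
; Firing plays a sound and spawns the projectile at the tank's DirectionArrow transform, then sets a CoolDown flag that a timer event clears after a few seconds.
; Started fires immediately without checking the cooldown, while Triggered repeats the same firing path only when the cooldown is clear.
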(event Custom|End%20Cool%20Down
  (Variables|Default|SetCool%20Down false))

(event EventStarted
  (bind _mytank (Variables|Default|GetMyTank))
  (bind _directionarrow (Variables|/Game/Blueprints/BP_PlayerCharacter.BP_PlayerCharacter_C|GetDirectionArrow _mytank))
  (bind _returnvalue (Transformation|GetWorldLocation _directionarrow))
  (Audio|PlaySoundatLocation "/Game/StudentWork/Effects/SFX/mixkit-falling-on-foil-748.mixkit-falling-on-foil-748" _returnvalue "0, 0, 0" 1.0 1.0 0.0 0 0 0 0)
  (Game|SpawnActorfromClass "/Game/StudentWork/Weapons/BP_Player_Bubble_Projectile.BP_Player_Bubble_Projectile_C" (Math|Transform|MakeTransform _returnvalue (Transformation|GetWorldRotation _directionarrow) "1.000000,1.000000,1.000000") "Undefined" "MultiplyWithRoot" 0 0)
  (Variables|Default|SetCool%20Down true)
  (Utilities|Time|SetTimerbyEvent (delegate Custom|End%20Cool%20Down) 3.0))

(event EventTriggered
  (bind _mytank (Variables|Default|GetMyTank))
  (bind _directionarrow (Variables|/Game/Blueprints/BP_PlayerCharacter.BP_PlayerCharacter_C|GetDirectionArrow _mytank))
  (bind _returnvalue (Transformation|GetWorldLocation _directionarrow))
  (if (not (Variables|Default|GetCool%20Down))
    (Audio|PlaySoundatLocation "/Game/StudentWork/Effects/SFX/mixkit-falling-on-foil-748.mixkit-falling-on-foil-748" _returnvalue "0, 0, 0" 1.0 1.0 0.0 0 0 0 0)
    (Game|SpawnActorfromClass "/Game/StudentWork/Weapons/BP_Player_Bubble_Projectile.BP_Player_Bubble_Projectile_C" (Math|Transform|MakeTransform _returnvalue (Transformation|GetWorldRotation _directionarrow) "1.000000,1.000000,1.000000") "Undefined" "MultiplyWithRoot" 0 0)
    (Variables|Default|SetCool%20Down true)
    (Utilities|Time|SetTimerbyEvent (delegate Custom|End%20Cool%20Down) 3.0)))

(fn ConstructionScript
  (|CallParentFunction))