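; BP_Turret is an enemy turret that fires projectiles and can be destroyed by damage.
; On BeginPlay it sets Health to Maxhealth and, if IsAutomatic is set, starts a looping timer for FireProjectile.
; FireProjectile spawns BP_Enemy_Projectile at the Arrow component's location and rotation.
; AnyDamage calls ApplyDamage without a target, subtracts the damage from Health, and destroys the actor at zero or below.
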(event Custom|Fire%20Projectile
  (bind _arrow (Variables|Default|GetArrow))
  (Game|SpawnActorfromClass "/Game/StudentWork/BP_Enemy_Projectile.BP_Enemy_Projectile_C" (Math|Transform|MakeTransform (Transformation|GetWorldLocation _arrow) (Transformation|GetWorldRotation _arrow) "1.000000,1.000000,1.000000") "Undefined" "MultiplyWithRoot" 0 0))

(event Game|Damage|EventAnyDamage
  (params (Damage :type Float%20%28single-precision%29) (DamageType :type Damage%20Type%20Object%20Reference) (InstigatedBy :type Controller%20Object%20Reference) (DamageCauser :type Actor%20Object%20Reference))
  (Game|Damage|ApplyDamage 0 Damage 0 0)
  (Variables|Default|SetHealth (- (Variables|Default|GetHealth) Damage))
  (if (<= (Variables|Default|GetHealth) 0.0)
    (Actor|DestroyActor)))

(event EventBeginPlay
  (Variables|Default|SetHealth (Variables|Default|GetMaxhealth))
  (if (Variables|Default|GetIs%20Automatic)
    (bind _returnvalue (Utilities|Time|SetTimerbyEvent (delegate Custom|Fire%20Projectile) 1.0 true))
    (Variables|Default|SetTimer _returnvalue)))

(fn ConstructionScript)