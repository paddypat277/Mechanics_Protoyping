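; BP_Enemy_Chase is an enemy Blueprint that pursues the player and attacks with projectiles.
; Its Move event uses AI MoveTo to approach the player character reference when valid, stopping within a small acceptance radius.
; Its AttackTarget event spawns a BP_Enemy_Projectile at the DirectionalArrow component's world location and rotation.
; The construction script only calls the parent's.
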(event EventAttackTarget
  (bind _directional_arrow (Variables|Default|GetDirectional%20arrow))
  (Game|SpawnActorfromClass "/Game/StudentWork/BP_Enemy_Projectile.BP_Enemy_Projectile_C" (Math|Transform|MakeTransform (Transformation|GetWorldLocation _directional_arrow) (Transformation|GetWorldRotation _directional_arrow) "1.000000,1.000000,1.000000") "Undefined" "MultiplyWithRoot" 0 0))

(event EventMove
  (bind _as_bp_player_character (Variables|Default|GetAs%20BP%20Player%20Character))
  (Utilities|IsValid _as_bp_player_character
    (:Is%20Valid
      (AI|AIMoveTo self "0, 0, 0" _as_bp_player_character 5e+01 false))))

(fn ConstructionScript
  (|CallParentFunction))