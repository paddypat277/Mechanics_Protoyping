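; Waypoint enemy Blueprint that patrols a list of target points while aiming its head at the player.
; Move sends the pawn via AI MoveTo to the current point, then increments the index on success, resetting it once it exceeds the array length.
; Tick rotates the head toward the player character with a look-at rotation and calls HullToFace, which is defined outside these graphs.
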(event Custom|Aim%20at%20Player
  (bind _as_bp_player_character (Variables|Default|GetAs%20BP%20Player%20Character))
  (bind _head (Variables|Default|GetHead))
  ;[1 1 1 0.5] Aim Turret at Player
  (Utilities|IsValid _as_bp_player_character
    (:Is%20Valid
      (Transformation|SetWorldRotation _head (Math|Rotator|FindLookatRotation (Transformation|GetWorldLocation _head) (Transformation|GetWorldLocation (Variables|/Script/Engine.Actor|GetRootComponent _as_bp_player_character))) false false))))

(event EventMove
  (AI|AIMoveTo self "0, 0, 0" (Utilities|Array|Get(acopy) (Variables|Default|GetMy%20Points) (Variables|Default|GetCurrent%20Index)) 5.0 false
    (:OnSuccess
      (Math|Integer|IncrementInt (Variables|Default|GetCurrent%20Index)
        (:%20%20
          (if (> (Variables|Default|GetCurrent%20Index) (Utilities|Array|Length (Variables|Default|GetMy%20Points)))
            (Variables|Default|SetCurrent%20Index 0)))))))

(event EventTick
  (params (DeltaSeconds :type Float%20%28single-precision%29))
  (CallFunction|AimatPlayer)
  (CallFunction|HulltoFace))

(fn ConstructionScript
  (|CallParentFunction))