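; BP_Enemy_Chaser is an enemy pawn that pursues the player and fires projectiles.
; Its Move event uses AI MoveTo toward the stored player character's current location with a small acceptance radius.
; Its AttackTarget event spawns BP_Enemy_Projectile at the location and rotation of its DirectionalArrow.
; The graph holds only these two behaviours, with no timing or trigger logic, and construction defers to the parent.
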(event EventMove
  (AI|AIMoveTo self (.location (Transformation|GetActorTransform (Variables|Default|GetAs%20BP%20Player%20Character))) 0 15.0 false))

(event EventAttackTarget
  (bind _directional_arrow (Variables|Default|GetDirectional%20arrow))
  (Game|SpawnActorfromClass "/Game/StudentWork/BP_Enemy_Projectile.BP_Enemy_Projectile_C" (Math|Transform|MakeTransform (Transformation|GetWorldLocation _directional_arrow) (Transformation|GetWorldRotation _directional_arrow) "1.000000,1.000000,1.000000") "Undefined" "MultiplyWithRoot" 0 0))

(fn ConstructionScript
  (|CallParentFunction))