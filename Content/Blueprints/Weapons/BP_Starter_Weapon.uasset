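; BP_Starter_Weapon is a tank weapon that spawns BP_Projectile actors at the location and rotation of the owning tank's direction arrow.
; When started, it checks the tank's BurstMode flag and either fires a single projectile or plays a timeline.
; In burst mode, both the timeline's update pin and an event track lead to the projectile spawn, so shots repeat while it plays.
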(event Custom|Fire
  (bind _mytank (Variables|Default|GetMyTank))
  (bind _directionarrow (Variables|/Game/Blueprints/BP_PlayerCharacter.BP_PlayerCharacter_C|GetDirectionArrow _mytank))
  (Game|SpawnActorfromClass "/Game/StudentWork/BP_Projectile.BP_Projectile_C" (Math|Transform|MakeTransform (Transformation|GetWorldLocation _directionarrow) (Transformation|GetWorldRotation _directionarrow) "1.000000,1.000000,1.000000") "Undefined" "MultiplyWithRoot" 0 0))

(event EventStarted
  (bind _mytank (Variables|Default|GetMyTank))
  (bind _directionarrow (Variables|/Game/Blueprints/BP_PlayerCharacter.BP_PlayerCharacter_C|GetDirectionArrow _mytank))
  (if (Variables|/Game/Blueprints/BP_PlayerCharacter.BP_PlayerCharacter_C|GetBurstMode _mytank)
    (Timeline|Timeline Play
      (:Update
        (Game|SpawnActorfromClass "/Game/StudentWork/BP_Projectile.BP_Projectile_C" (Math|Transform|MakeTransform (Transformation|GetWorldLocation _directionarrow) (Transformation|GetWorldRotation _directionarrow) "1.000000,1.000000,1.000000") "Undefined" "MultiplyWithRoot" 0 0 :!label _label))
      (:NewTrack_2
        (CallFunction|Fire)))
    (else
      (goto _label))))

(fn ConstructionScript
  (|CallParentFunction))